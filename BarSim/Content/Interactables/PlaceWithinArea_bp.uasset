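; An interactable placement area, shown by a colored decal and bounded by a sphere, that reports when an actor is placed in it.
; On BeginPlay, a shared Radius sizes both the decal and the sphere, and a dynamic material instance tints the decal amber.
; The PlaceSomethingHere event forwards the placed actor through the SomethingWasPlaced dispatcher, with no range check or other placement logic of its own.
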(event `self.ReceiveBeginPlay`
  (bind _radius (`self.Radius`))
  (`SceneComponent.SetRelativeScale3D` (`self.Decal`) (`KismetMathLibrary.MakeVector` 1.0 _radius _radius))
  (`SphereComponent.SetSphereRadius` (`self.Sphere`) (`self.Radius`) true)
  (bind _returnvalue (`DecalComponent.CreateDynamicMaterialInstance` (`self.Decal`)))
  (bind _output_get (set `self.DecalMaterial` _returnvalue))
  (`MaterialInstanceDynamic.SetVectorParameterValue` _output_get "Color" (struct :`R` 0.65625 :`G` 0.404055 :`B` 0.057334 :`A` 1.0)))

(event `PlaceSomethingHere`
  (params (Actor :type "Actor Object Reference"))
  (`self.SomethingWasPlaced` Actor))

(fn `UserConstructionScript`)